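; BP_TestGun2Actor is a test hitscan gun whose ExecuteFire takes a fire context and always returns true.
; It uses two Visibility traces: one along the context's aim to find the aim point, then one from the muzzle slightly past that point, drawn for debugging.
; Only a muzzle-trace hit receives damage, using the context's amount and instigator, so obstructions in front of the barrel take the shot.
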(fn `ExecuteFire`
  (params (FireContext :type "GunFireContext Structure (by ref)"))
  (returns (ReturnValue :type Boolean))
  (bind _aimignoreactorlist (`self.AimIgnoreActorList`))
  (bind (_shooter _instigatorcontroller _aimorigin _aimdirection _damage) (break `GunFireContext` (`self.GunFireContext`)))
  (bind _output_get (set `self.GunFireContext` FireContext))
  (set `self.AimDirection` (`KismetMathLibrary.Normal` (`.AimDirection` (break `GunFireContext` _output_get))))
  (bind _output_get_2 (set `self.AimTraceStart` (`.AimOrigin` (break `GunFireContext` (`self.GunFireContext`)))))
  (set `self.AimTraceEnd` (+ _output_get_2 (* (`self.AimDirection`) (`self.HitscanRange`))))
  (`KismetArrayLibrary.Array_Add` _aimignoreactorlist self)
  (`KismetArrayLibrary.Array_Add` _aimignoreactorlist (`.Shooter` (break `GunFireContext` (`self.GunFireContext`))))
  (bind _outhit (`KismetSystemLibrary.LineTraceSingle` (`self.AimTraceStart`) (`self.AimTraceEnd`) "TraceTypeQuery1" false _aimignoreactorlist "None" true (struct :`R` 1.0 :`A` 1.0) (struct :`G` 1.0 :`A` 1.0) 0.3))
  (bind (_bblockinghit _binitialoverlap _time _distance _location _impactpoint) (`GameplayStatics.BreakHitResult` _outhit))
  (if _bblockinghit
    (set `self.AimPoint` _impactpoint)
    (else
      (set `self.AimPoint` (`self.AimTraceEnd`))))
  (set `self.MuzzleTraceStart` (`SceneComponent.K2_GetComponentLocation` (`self.Muzzle`)))
  (bind _output_get_3 (set `self.MuzzleDirection` (`KismetMathLibrary.Normal` (- (`self.AimPoint`) (`self.MuzzleTraceStart`)))))
  (if (`KismetMathLibrary.Vector_IsNearlyZero` _output_get_3)
    (set `self.MuzzleDirection` (`self.AimDirection`)))
  (set `self.MuzzleTraceEnd` (+ (`self.AimPoint`) (* (`self.MuzzleDirection`) 10.0)))
  (bind _outhit_2 (`KismetSystemLibrary.LineTraceSingle` (`self.MuzzleTraceStart`) (`self.MuzzleTraceEnd`) "TraceTypeQuery1" false (`self.AimIgnoreActorList`) "ForDuration" true (struct :`R` 1.0 :`A` 1.0) (struct :`G` 1.0 :`A` 1.0) 1.2))
  (bind (_bblockinghit_2 _binitialoverlap_2 _time_2 _distance_2 _location_2 _impactpoint_2 _normal _impactnormal _physmat _hitactor) (`GameplayStatics.BreakHitResult` _outhit_2))
  (if _bblockinghit_2
    (`GameplayStatics.ApplyDamage` _hitactor _damage _instigatorcontroller self))
  (return true))

(fn `UserConstructionScript`)