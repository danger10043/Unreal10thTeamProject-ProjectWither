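; Boss gorilla monster Blueprint that sets up the boss's attack hitboxes.
; On BeginPlay it registers the Back, LeftArm, RightArm and Saw hitboxes with its MonsterComponent, each under a matching name.
; The graph holds no other logic, and the construction script is empty.
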(event `self.ReceiveBeginPlay`
  (`MonsterComponent.RegisterAttackHitbox` (`self.MonsterComponent`) "Back" (`self.Back`))
  (`MonsterComponent.RegisterAttackHitbox` (`self.MonsterComponent`) "LeftArm" (`self.LeftArm`))
  (`MonsterComponent.RegisterAttackHitbox` (`self.MonsterComponent`) "RightArm" (`self.RightArm`))
  (`MonsterComponent.RegisterAttackHitbox` (`self.MonsterComponent`) "Saw" (`self.Saw`)))

(fn `UserConstructionScript`)