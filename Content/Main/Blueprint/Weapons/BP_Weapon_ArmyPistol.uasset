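; Army pistol weapon Blueprint that implements hitscan firing through ExecuteFire; its event graph and construction script are empty.
; A Visibility trace from the fire context's camera aim finds the target point, then a second trace from the muzzle toward it decides the actual hit.
; Hits within FireRange of the pistol receive the context's damage and a Niagara impact effect.
; Every shot spawns a muzzle effect and reports ammo consumed.
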(event `self.ReceiveBeginPlay`)

(fn `ExecuteFire`
  (params (FireContext :type "GunFireContext Structure (by ref)"))
  (returns (bOutConsumeAmmo :type Boolean) (ReturnValue :type Boolean))
  (bind _muzzle (`self.Muzzle`))
  (bind _aimignoreactorlist (`self.AimIgnoreActorList`))
  (bind (_shooter _instigatorcontroller _aimorigin _aimdirection _damage) (break `GunFireContext` (`self.GunFireContext`)))
  (bind _returnvalue (`SceneComponent.GetForwardVector` _muzzle))
  (set `self.GunFireContext` FireContext)
  (`|ExecutionSequence`
    (:`then_0`
      ; 카메라에서 발사한 Line Trace가 닿은 목표 지점 계산
      (set `self.AimDirection` (`KismetMathLibrary.Normal` (`.AimDirection` (break `GunFireContext` (`self.GunFireContext`)))))
      (bind _output_get (set `self.AimTraceStart` (`.AimOrigin` (break `GunFireContext` (`self.GunFireContext`)))))
      (set `self.AimTraceEnd` (+ _output_get (* (`self.AimDirection`) (`self.HitscanRange`))))
      (`KismetArrayLibrary.Array_Add` _aimignoreactorlist self)
      (`KismetArrayLibrary.Array_Add` _aimignoreactorlist (`.Shooter` (break `GunFireContext` (`self.GunFireContext`))))
      (bind _outhit (`KismetSystemLibrary.LineTraceSingle` (`self.AimTraceStart`) (`self.AimTraceEnd`) "TraceTypeQuery1" false _aimignoreactorlist "None" true (struct :`R` 1.0 :`A` 1.0) (struct :`G` 1.0 :`A` 1.0) 0.3))
      (bind (_bblockinghit _binitialoverlap _time _distance _location _impactpoint) (`GameplayStatics.BreakHitResult` _outhit))
      (if _bblockinghit
        (set `self.AimPoint` _impactpoint)
        (else
          (set `self.AimPoint` (`self.AimTraceEnd`)))))
    (:`then_1`
      (bind _returnvalue_2 (`NiagaraFunctionLibrary.SpawnSystemAtLocation` "/Game/Main/VFX/Player/NS_Fire_Weapon_ArmyPistol.NS_Fire_Weapon_ArmyPistol" (+ (`SceneComponent.K2_GetComponentLocation` _muzzle) (* _returnvalue 100.0)) (`KismetMathLibrary.Conv_VectorToRotator` _returnvalue) (0.9 0.9 0.9)))
      (`NiagaraComponent.SetForceSolo` _returnvalue_2 true)
      (`NiagaraComponent.SetCustomTimeDilation` _returnvalue_2 2.0))
    (:`then_2`
      ; 카메라에서 발사한 Line Trace의 타겟 지점에 실제 총구 위치로부터 Line Trace 발사 후 데미지 판정
      (set `self.MuzzleTraceStart` (`SceneComponent.K2_GetComponentLocation` (`self.Muzzle`)))
      (bind _output_get_2 (set `self.MuzzleDirection` (`KismetMathLibrary.Normal` (- (`self.AimPoint`) (`self.MuzzleTraceStart`)))))
      (if (`KismetMathLibrary.Vector_IsNearlyZero` _output_get_2)
        (set `self.MuzzleDirection` (`self.AimDirection`)))
      (set `self.MuzzleTraceEnd` (+ (`self.AimPoint`) (* (`self.MuzzleDirection`) 10.0)))
      (bind _outhit_2 (`KismetSystemLibrary.LineTraceSingle` (`self.MuzzleTraceStart`) (`self.MuzzleTraceEnd`) "TraceTypeQuery1" false (`self.AimIgnoreActorList`) "None" true (struct :`R` 1.0 :`A` 1.0) (struct :`G` 1.0 :`A` 1.0) 1.2))
      (bind (_bblockinghit_2 _binitialoverlap_2 _time_2 _distance_2 _location_2 _impactpoint_2 _normal _impactnormal _physmat _hitactor) (`GameplayStatics.BreakHitResult` _outhit_2))
      (if (and _bblockinghit_2 (<= (`KismetMathLibrary.Vector_DistanceSquared` (`self.K2_GetActorLocation`) _location_2) (`KismetMathLibrary.Square` (`self.FireRange`))))
        (`GameplayStatics.ApplyDamage` _hitactor _damage _instigatorcontroller self)
        (`NiagaraFunctionLibrary.SpawnSystemAtLocation` "/Game/Main/VFX/Player/NS_Hit_Weapon_ArmyPistol.NS_Hit_Weapon_ArmyPistol" _location_2 (struct) (0.7 0.7 0.7)))
      (return true true))))

(fn `UserConstructionScript`)